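; Parent Blueprint for interactable resource objects that turn into a spawned actor when used.
; The Interact event calls InteractedWith, which spawns the SpawnObj class 150 units above the resource with its rotation and scale, then destroys the resource.
; A getter exposes TimeToDestroy, though the interaction here does not use it.
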(event EventInteract
  (CallFunction|Interactedwith))

(fn ConstructionScript)

(fn Interactedwith
  (bind _self self)
  (bind _returnvalue (Transformation|GetActorTransform _self))
  (Game|SpawnActorfromClass (Variables|Default|GetSpawnObj) (Math|Transform|MakeTransform (Math|Vector|MakeVector (.x (.location _returnvalue)) (.y (.location _returnvalue)) (+ (.z (.location _returnvalue)) 1.5e+02)) (.rotation _returnvalue) (.scale _returnvalue)) "Undefined" 0 0)
  (Actor|DestroyActor))

(fn GetTimetoDestroy
  (return (Variables|Default|GetTimeToDestroy)))